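; BP_GM is a manager Blueprint that runs the opening menu and photo-upload flow, then sets up the player's gambler character.
; It swaps UI_Main for UI_UploadPhoto through click event bindings, tracking the active widget in CurrentView.
; When upload finishes, it stores the front and side pictures and gender, then finds the male and female player BP_Gambler actors.
; The gender-matching actor receives the face data, and the other becomes an opponent.
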(event `self.ReceiveBeginPlay`
  (bind _returnvalue (`|CreateWidget` "/Game/UI/UI_Main.UI_Main_C"))
  (bind _output_get (set `self.CurrentView` _returnvalue))
  (`UserWidget.AddToViewport` _output_get 0)
  (add `/Game/UI/UI_Main.OnStartClicked` _returnvalue (delegate `OnStartClicked_Event`)))

(event `OnStartClicked_Event`
  (`Widget.RemoveFromParent` (`self.CurrentView`))
  (bind _returnvalue (`|CreateWidget` "/Game/UI/UI_UploadPhoto.UI_UploadPhoto_C"))
  (bind _output_get (set `self.CurrentView` _returnvalue))
  (`UserWidget.AddToViewport` _output_get 0)
  (add `/Game/UI/UI_UploadPhoto.OnDoneClicked` _returnvalue (delegate `OnDoneClicked_Event`)))

(event `OnDoneClicked_Event`
  (params (FrontPicture :type "Texture2D Object Reference") (LeftSidePicture :type "Texture2D Object Reference") (RightSidePicture :type "Texture2D Object Reference") (Gender :type "/Game/Blueprints/Enum_Gender Enum" :default "NewEnumerator0"))
  (bind (_selectedface_frontpicture _selectedface_leftsidepicture _selectedface_rightsidepicture _selectedface_gender) (break `/Game/Blueprints/Struct_Face` (`self.SelectedFace`)))
  (bind _femaleplayeractor (`self.FemalePlayerActor`))
  (bind _maleplayeractor (`self.MalePlayerActor`))
  (set `self.SelectedFace` (make `/Game/Blueprints/Struct_Face` FrontPicture LeftSidePicture RightSidePicture Gender))
  (`Widget.RemoveFromParent` (`self.CurrentView`))
  (bind _outactors (`GameplayStatics.GetAllActorsOfClass` "/Game/Blueprints/BP_Gambler.BP_Gambler_C"))
  (for _array_element _outactors
    (if (`/Game/Blueprints/BP_Gambler.bIsPlayer` _array_element)
      (switch `/Game/Blueprints/Enum_Character` (`/Game/Blueprints/BP_Gambler.CharacterType` _array_element)
        (:`NewEnumerator0`
          (set `self.MalePlayerActor` _array_element :!label _label))
        (:`NewEnumerator1`
          (goto _label))
        (:`NewEnumerator2`
          (set `self.FemalePlayerActor` _array_element :!label _label_2))
        (:`NewEnumerator3`
          (goto _label_2)))))
  (switch `/Game/Blueprints/Enum_Gender` _selectedface_gender
    (:`NewEnumerator0`
      (`/Game/Blueprints/BP_Gambler.MakeOpponent` _femaleplayeractor)
      (set `self.SelectedPlayerActor` _maleplayeractor))
    (:`NewEnumerator1`
      (`/Game/Blueprints/BP_Gambler.MakeOpponent` _maleplayeractor)
      (set `self.SelectedPlayerActor` _femaleplayeractor)))
  (`/Game/Blueprints/BP_Gambler.FaceSelected` (`self.SelectedPlayerActor`) (`self.SelectedFace`)))

(fn `UserConstructionScript`)