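; BP_Randomness_Manager is a Blueprint that periodically reshuffles a pool of values and hands them out as random, unique picks.
; Tick accumulates delta time, and every ten seconds shuffles the Case1 value array, resets the read index and fires the Case1TimeHasCome call.
; An allocation function advances the index and returns the next entry, so picks do not repeat between shuffles, with no bounds check on the index.
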(event `self.ReceiveTick`
  (params (DeltaSeconds :type "Float (single-precision)"))
  (bind _output_get (set `self.Case1_Counter` (+ DeltaSeconds (`self.Case1_Counter`))))
  (if (>= _output_get 10.0)
    (set `self.Case1_Counter` 0.0)
    (`KismetArrayLibrary.Array_Shuffle` (`self.Case1_AllocatedValues`))
    (set `self.Case1_CurrentIndex` -1)
    (`self.Case1_TimeHasCome`)))

(fn `Case1_AllocateRandomUniqueValue`
  (returns (Value :type Integer))
  (bind _output_get (set `self.Case1_CurrentIndex` (+ (`self.Case1_CurrentIndex`) 1)))
  (return (`|GetArrayItem` (`self.Case1_AllocatedValues`) _output_get)))

(fn `UserConstructionScript`)