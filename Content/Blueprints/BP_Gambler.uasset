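; BP_Gambler is a gambler character that serves as either the player or an opponent, with a selectable face.
; The construction script picks one of four body meshes by CharacterType, attaches HeadMesh to the Head socket and creates its dynamic face material.
; BeginPlay applies the role, forwarding IsPlayer to AB_Gambler and showing the head only for the player.
; FaceSelected swaps the face texture; Tick is an empty stub.
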(event `self.ReceiveTick`
  (params (DeltaSeconds :type "Float (single-precision)"))
  ;[1 1 1] Face replacement logic comes here
  ;;[1 1 1] Feed the data per tick, somehow
)

(event `FaceSelected`
  (params (Face :type "/Game/Blueprints/Struct_Face Structure"))
  (bind _output_get (set `self.SelectedFace` Face))
  ;[1 1 1] Face replacement logic comes here
  (`MaterialInstanceDynamic.SetTextureParameterValue` (`self.FaceMaterialInstance`) "FaceTexture" (`.FrontPicture_2_052795DC41D6C75F83380A838A20DBC4` (break `/Game/Blueprints/Struct_Face` _output_get))))

(event `MakePlayer`
  (set `self.bIsPlayer` true)
  (bind _asab_gambler (cast `/Game/Animations/AB_Gambler` (`SkeletalMeshComponent.GetAnimInstance` (`self.SkeletalMesh`))))
  (set `/Game/Animations/AB_Gambler.bIsPlayer` true _asab_gambler)
  (`SceneComponent.SetHiddenInGame` (`self.HeadMesh`) false false))

(event `MakeOpponent`
  (set `self.bIsPlayer` false)
  (bind _asab_gambler (cast `/Game/Animations/AB_Gambler` (`SkeletalMeshComponent.GetAnimInstance` (`self.SkeletalMesh`))))
  (set `/Game/Animations/AB_Gambler.bIsPlayer` false _asab_gambler)
  (`SceneComponent.SetHiddenInGame` (`self.HeadMesh`) true false))

(event `self.ReceiveBeginPlay`
  (if (`self.bIsPlayer`)
    (`self.MakePlayer`)
    (else
      (`self.MakeOpponent`))))

(fn `UserConstructionScript`
  (`SkinnedMeshComponent.SetSkinnedAssetAndUpdate` (`self.SkeletalMesh`) (select `/Game/Blueprints/Enum_Character` (`self.CharacterType`) :`NewEnumerator0` "/Game/Meshes/SkeletalMeshes/M_Actor1.M_Actor1" :`NewEnumerator1` "/Game/Meshes/SkeletalMeshes/M_Actor2.M_Actor2" :`NewEnumerator2` "/Game/Meshes/SkeletalMeshes/F_Actor1.F_Actor1" :`NewEnumerator3` "/Game/Meshes/SkeletalMeshes/F_Actor2.F_Actor2" :!type "SkeletalMesh Object Reference") true)
  (`SceneComponent.K2_AttachToComponent` (`self.HeadMesh`) (`self.SkeletalMesh`) "Head" "KeepRelative" "KeepRelative" "KeepWorld" false)
  (bind _returnvalue (`PrimitiveComponent.CreateDynamicMaterialInstance` (`self.HeadMesh`) 0 "/Game/Materials/M_Face.M_Face" "None"))
  (set `self.FaceMaterialInstance` _returnvalue))